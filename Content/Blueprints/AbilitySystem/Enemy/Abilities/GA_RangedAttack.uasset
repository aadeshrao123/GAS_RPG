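; Enemy ranged attack gameplay ability that fires a projectile at the avatar's combat target.
; On activation it turns the avatar toward the target and plays a random tagged attack montage.
; A gameplay event matching the montage's tag draws a debug sphere at that tag's combat socket, spawns the projectile toward the target's current location, then ends the ability after a short delay.
; Montage completion, interruption or cancellation also ends the ability.
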(event Ability|EventActivateAbility
  (bind _returnvalue (Ability|GetAvatarActorfromActorInfo))
  (bind _returnvalue_2 (Class|EnemyInterface|GetCombatTarget(Message) (Ability|GetAvatarActorfromActorInfo)))
  (Class|CombatInterface|UpdateFacingTarget(Message) _returnvalue (Transformation|GetActorLocation _returnvalue_2))
  (bind _returnvalue_3 (Class|CombatInterface|GetAttackMontage(Message) _returnvalue))
  (bind _output_get (Variables|Default|SetTaggedMontage (Class|RPGDamageGamaplayAbility|GetRandomTaggedMontages _returnvalue_3)))
  (|PlayMontageandWaitProxy "None" (.Montage (Utilities|Struct|BreakTaggedMontage _output_get)) 1.0 "None" false 1.0 0.0 false
    (:then
      (Ability|Tasks|WaitGameplayEvent (.MontageTag (Utilities|Struct|BreakTaggedMontage _output_get)) 0
        (:EventReceived
          (bind _returnvalue_4 (Class|CombatInterface|GetCombatSocketLocation(Message) (Ability|GetAvatarActorfromActorInfo) (.MontageTag (Utilities|Struct|BreakTaggedMontage _output_get))))
          (Rendering|Debug|DrawDebugSphere _returnvalue_4 5.0 12 "(R=1.000000,G=0.000000,B=0.000000,A=1.000000)" 0.5)
          (bind _returnvalue_5 (Class|EnemyInterface|GetCombatTarget(Message) (Ability|GetAvatarActorfromActorInfo)))
          (Class|RPGProjectileSpell|SpawnProjectile (Transformation|GetActorLocation _returnvalue_5))
          (Utilities|FlowControl|Delay 1.0)
          (Ability|EndAbility))))
    (:OnCompleted
      (Ability|EndAbility :!label _label))
    (:OnInterrupted
      (goto _label))
    (:OnCancelled
      (goto _label))))