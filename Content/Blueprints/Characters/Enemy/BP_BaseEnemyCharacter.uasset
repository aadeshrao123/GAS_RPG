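; Base enemy character Blueprint that supplies the visual effects and warp targeting for enemies.
; On BeginPlay, after the parent logic, a timeline scales the mesh.
; Separate timelines drive the Dissolve parameter on dynamic material instances passed in for the mesh and weapon.
; UpdateFacingTarget sets the "FacingTarget" Motion Warping target from a given location.
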(event EventBeginPlay
  (|CallParentFunction)
  (bind _scaletrack (Timeline|ScaleTimeline PlayFromStart)
    (:Update
      (Transformation|SetRelativeScale3D (Variables|Character|GetMesh) (Math|Conversions|ToVector(Float) _scaletrack)))))

(event EventStartDissolveMaterialTimelineMesh
  (params (DynamicMaterialInstance :type Material%20Instance%20Dynamic%20Object%20Reference))
  (bind _dissolvetrack (Timeline|Timeline Play)
    (:Update
      (Rendering|Material|SetScalarParameterValue DynamicMaterialInstance "Dissolve" _dissolvetrack :!class /Script/Engine.MaterialInstanceDynamic))))

(event EventUpdateFacingTarget
  (params (Target :type Vector%20%28by%20ref%29 :default "0, 0, 0"))
  (Class|MotionWarpingComponent|AddorUpdateWarpTargetfromLocation (Variables|Default|GetMotionWarping) "FacingTarget" Target))

(event EventStartDissolveMaterialTimelineWeapon
  (params (DynamicMaterialInstance :type Material%20Instance%20Dynamic%20Object%20Reference))
  (bind _weapondissolvetrack (Timeline|Timeline_0 Play)
    (:Update
      (Rendering|Material|SetScalarParameterValue DynamicMaterialInstance "Dissolve" _weapondissolvetrack :!class /Script/Engine.MaterialInstanceDynamic))))

(fn ConstructionScript)